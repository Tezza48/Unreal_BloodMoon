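; Base camera actor that keeps its CameraComponent aimed at a Target actor.
; LookAtTarget runs in the construction script and every Tick, rotating the camera from the actor's location toward the target.
; Tick also hides CamMeshHolder and its children while the player's view location matches the camera's, so the mesh only shows from other viewpoints.
; A pitch clamp using MinPitch and MaxPitch exists but is unconnected.
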(event EventBeginPlay)

(event Collision|EventActorBeginOverlap
  (params (OtherActor :type Actor%20Object%20Reference)))

(event EventTick
  (params (DeltaSeconds :type Float%20%28single-precision%29))
  (bind _cammeshholder (Variables|Default|GetCamMeshHolder))
  (CallFunction|LookatTarget)
  (if (Math|Vector|Equal(Vector) (.OutLocation (Actor|GetActorEyesViewPoint (Game|GetPlayerCameraManager 0))) (Transformation|GetWorldLocation (Variables|CameraActor|GetCameraComponent)) 0.0001)
    (Rendering|SetVisibility _cammeshholder false true)
    (else
      (Rendering|SetVisibility _cammeshholder true true))))

(fn ConstructionScript
  (CallFunction|LookatTarget))

(fn LookatTarget
  (Transformation|SetWorldRotation (Variables|CameraActor|GetCameraComponent) (Math|Rotator|FindLookatRotation (Transformation|GetActorLocation) (Transformation|GetActorLocation (Variables|Default|GetTarget))) false false))