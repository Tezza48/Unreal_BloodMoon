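; AI controller for enemies that runs the BT_Enemy behavior tree when play begins.
; When its PawnSensing component sees a BP_Character, it writes that character's world position to the blackboard's Location key.
; An unconnected node chain that would write the player character's position to the same key is left in the graph and never runs.
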(event OnSeePawn(PawnSensing)
  (params (Pawn :type Pawn%20Object%20Reference))
  (bind _asbp_character (Utilities|Casting|CastToBP_Character Pawn))
  (AI|Components|Blackboard|SetValueasVector (AI|GetBlackboard 0) (Utilities|Name|MakeLiteralName "Location") (Transformation|GetActorLocation _asbp_character)))

(event EventBeginPlay
  (AI|RunBehaviorTree "/Game/Blueprints/AI/BT_Enemy.BT_Enemy"))

(event EventTick
  (params (DeltaSeconds :type Float%20%28single-precision%29)))

(fn ConstructionScript)