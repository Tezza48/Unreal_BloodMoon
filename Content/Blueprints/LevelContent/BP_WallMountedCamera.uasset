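; Wall-mounted camera that becomes the player's view when a linked trigger volume is entered.
; On BeginPlay it points its child BP_TargetedCamera at the player character and binds to the trigger's begin-overlap event.
; Any overlap, or the player starting inside the volume, switches the view target to that camera.
; The overlap handler does not filter by actor, and nothing here restores the previous view.
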(event Custom|SetThisToMainCamera
  (params (OverlappedActor :type Actor%20Object%20Reference) (OtherActor :type Actor%20Object%20Reference))
  (Game|Player|SetViewTargetwithBlend (Game|GetPlayerController 0) (Variables|/Script/Engine.ChildActorComponent|GetChildActor (Variables|Default|GetCamera)) 0.0 "VTBlend_Linear" 0.0 false))

(event EventBeginPlay
  (bind _triggervolume (Variables|Default|GetTriggerVolume))
  (bind _asbp_targeted_camera (Utilities|Casting|CastToBP_TargetedCamera (Variables|/Script/Engine.ChildActorComponent|GetChildActor (Variables|Default|GetCamera))))
  (Variables|/Game/Blueprints/BaseClasses/BP_TargetedCamera.BP_TargetedCamera_C|SetTarget _asbp_targeted_camera (Game|GetPlayerCharacter 0))
  (Collision|BindEventtoOnActorBeginOverlap _triggervolume (delegate Custom|SetThisToMainCamera))
  (if (Collision|IsOverlappingActor _triggervolume (Game|GetPlayerCharacter 0) :!class /Script/Engine.Actor)
    (Utilities|LookatPlayer)))

(event Collision|EventActorBeginOverlap
  (params (OtherActor :type Actor%20Object%20Reference)))

(event EventTick
  (params (DeltaSeconds :type Float%20%28single-precision%29)))

(fn ConstructionScript)