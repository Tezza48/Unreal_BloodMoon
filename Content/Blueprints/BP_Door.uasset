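; Door actor that animates DoorRoot between a closed and an open transform, with an option to start opened.
; The construction script captures the current transform as closed and applies the open one if StartOpened is set.
; OpenDoor and CloseDoor play or reverse a timeline that lerps the transforms.
; Trigger branches on IsOpen, but both events set that flag inversely, so repeated triggers repeat the same action.
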(event Custom|Event%20Open%20Door
  (Variables|Default|SetIsOpen false)
  (bind _alpha (Timeline|DoorOpening Play)
    (:Update
      (Transformation|SetRelativeTransform (Variables|Default|GetDoorRoot) (Math|Transform|Lerp(Transform) (Variables|Default|GetCloseTransform) (Variables|Default|GetOpenTransform) _alpha) false false))))

(event Custom|Event%20Close%20Door
  (Variables|Default|SetIsOpen true)
  (bind _alpha (Timeline|DoorOpening Reverse)
    (:Update
      (Transformation|SetRelativeTransform (Variables|Default|GetDoorRoot) (Math|Transform|Lerp(Transform) (Variables|Default|GetCloseTransform) (Variables|Default|GetOpenTransform) _alpha) false false))))

(event EventBeginPlay)

(event Collision|EventActorBeginOverlap
  (params (OtherActor :type Actor%20Object%20Reference)))

(event EventTick
  (params (DeltaSeconds :type Float%20%28single-precision%29)))

(event EventTrigger
  (if (Variables|Default|GetIsOpen)
    (CallFunction|EventCloseDoor)
    (else
      (CallFunction|EventOpenDoor))))

(fn ConstructionScript
  (Variables|Default|SetCloseTransform (Transformation|GetRelativeTransform (Variables|Default|GetDoorRoot)))
  (if (Variables|Default|GetStartOpened)
    (Transformation|SetRelativeTransform (Variables|Default|GetDoorRoot) (Variables|Default|GetOpenTransform) false false))
  (Variables|Default|SetIsOpen (Variables|Default|GetStartOpened)))